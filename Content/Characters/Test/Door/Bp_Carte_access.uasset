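; Access card pickup that raises the player knight's access level, presumably for doors.
; On overlap with BP_ThirdPersonKnight, it copies its card level to the player and destroys itself, only if that level exceeds the player's current one.
; The construction script colors the cube by level via NiveauAccessCouleur, then sets the "Base Color" material parameter to green or red for the first two levels.
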(event EventBeginPlay)

(event Collision|EventActorBeginOverlap
  (params (OtherActor :type Actor%20Object%20Reference))
  (bind _asbp_third_person_knight (Utilities|Casting|CastToBP_ThirdPersonKnight OtherActor))
  (if (< (Variables|/Game/ThirdPerson/Blueprints/BP_ThirdPersonKnight.BP_ThirdPersonKnight_C|GetPlayerNiveauAccess _asbp_third_person_knight) (Variables|Components|GetcarteNiveauAcces))
    (Variables|/Game/ThirdPerson/Blueprints/BP_ThirdPersonKnight.BP_ThirdPersonKnight_C|SetPlayerNiveauAccess _asbp_third_person_knight (Variables|Components|GetcarteNiveauAcces))
    (Actor|DestroyActor)))

(event EventTick
  (params (DeltaSeconds :type Float%20%28single-precision%29)))

(fn ConstructionScript
  (CallFunction|NiveauAccessCouleur (Variables|Components|GetcarteNiveauAcces) (Variables|Default|GetCube))
  (switch int (Variables|Components|GetcarteNiveauAcces)
    (:0
      (Rendering|Material|SetVectorParameterValueonMaterials (Variables|Default|GetCube) "Base Color" (Math|Conversions|ToVector(LinearColor) "(R=0.005677,G=0.218750,B=0.000000,A=1.000000)")))
    (:1
      (Rendering|Material|SetVectorParameterValueonMaterials (Variables|Default|GetCube) "Base Color" (Math|Conversions|ToVector(LinearColor) "(R=0.218750,G=0.009000,B=0.006824,A=1.000000)")))))